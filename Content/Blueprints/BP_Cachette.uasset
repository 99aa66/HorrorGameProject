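; BP_Cachette is an interactable hiding spot that moves the player into a hidden position.
; On BeginPlay it builds the target transform from HideTransform's location, halving the player's Z scale for short objects.
; Interaction disables player movement, then a timeline lerps the player to that transform while easing control yaw toward LookTransform.
; The HasDoor branch is empty, and no exit logic exists.
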(event `self.ReceiveBeginPlay`
  (if (`self.ShortObject`)
    (set `self.PlayerScale` 0.5)
    (else
      (set `self.PlayerScale` 1.0)))
  (set `self.ActorHideTransform` (`KismetMathLibrary.MakeTransform` (`SceneComponent.K2_GetComponentLocation` (`self.Hide_Transform`)) (struct) (`KismetMathLibrary.MakeVector` 1.0 1.0 (`self.PlayerScale`))))
  (if (`self.HasDoor ?`)
    _))

(event `/Game/Blueprints/BPI_Interaction.Interaction`
  (bind _ref_player (`self.Ref_Player`))
  (bind _returnvalue (`Pawn.GetController` _ref_player))
  (bind _returnvalue_2 (`Controller.GetControlRotation` _returnvalue))
  (bind (_returnvalue_roll _returnvalue_pitch _returnvalue_yaw) (`KismetMathLibrary.BreakRotator` (`KismetMathLibrary.RInterpTo` _returnvalue_2 (`KismetMathLibrary.FindLookAtRotation` (`SceneComponent.K2_GetComponentLocation` (`/Game/Blueprints/BP_Player.Camera` _ref_player)) (`SceneComponent.K2_GetComponentLocation` (`self.Look_Transform`))) (`GameplayStatics.GetWorldDeltaSeconds`))))
  (bind _asbp_player (cast `/Game/Blueprints/BP_Player` (`GameplayStatics.GetPlayerCharacter` 0)))
  (bind _output_get (set `self.Ref_Player` _asbp_player))
  (`CharacterMovementComponent.DisableMovement` (`Character.CharacterMovement` _output_get))
  (set `self.ActorCurrentTransform` (`self.GetTransform` _asbp_player))
  (bind (_direction _smooth_transition) (`Timeline|Timeline`)
    (:`Update`
      (`self.K2_SetActorTransform` _ref_player (`KismetMathLibrary.TLerp` (`self.ActorCurrentTransform`) (`self.ActorHideTransform`) _smooth_transition) false false)
      (`Controller.SetControlRotation` _returnvalue (`KismetMathLibrary.MakeRotator` (.roll _returnvalue_2) (.pitch _returnvalue_2) _returnvalue_yaw)))))

(fn `UserConstructionScript`)