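; Physics door that the player grabs and pushes or pulls with mouse movement.
; GrabDoor pins a grab point to the door mesh, stores player references and slows walking.
; While grabbed, Tick aims the camera arm at that point and builds a camera-relative force from mouse delta.
; Only forces above MaxForce are clamped and applied, scaled by mass, at the grab point; velocity-driven and center-of-mass alternatives are unused.
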(event `self.ReceiveTick`
  (params (DeltaSeconds :type "Float (single-precision)"))
  (bind _returnvalue (`GameplayStatics.GetPlayerController` 0))
  (bind _sm_door (`self.SM_Door`))
  (bind (_deltax _deltay) (`PlayerController.GetInputMouseDelta` _returnvalue))
  (bind _playercameramanager (`PlayerController.PlayerCameraManager` _returnvalue))
  (bind (_relativelocation_x _relativelocation_y _relativelocation_z) (`KismetMathLibrary.BreakVector` (`SceneComponent.RelativeLocation` (`self.DoorHandel`))))
  ;[1 1 1] Recup Mouse Input To Make the Movement
  (if (`self.Grabbed`)
    (`self.Lock look`)
    (set `self.MouseDeltaX` _deltax)
    (set `self.MouseDeltaY` _deltay)
    (bind _output_get (set `self.Force` (+ (* (* (* (`self.GetActorRightVector` _playercameramanager) (`self.MouseDeltaX`)) 200.0) (`PlayerController.GetDeprecatedInputYawScale` _returnvalue)) (* (* (* (`self.GetActorForwardVector` _playercameramanager) (`self.MouseDeltaY`)) 500.0) (* (`PlayerController.GetDeprecatedInputPitchScale` _returnvalue) -1.0)))))
    (set `self.Force` (`KismetMathLibrary.MakeVector` (.x _output_get) (.y _output_get) _relativelocation_z))
    ;[1 1 1] Lock The Max Force
    (if (> (`KismetMathLibrary.Vector_Distance` (`KismetMathLibrary.Vector_Zero`) (`self.Force`)) (`self.MaxForce`))
      (set `self.Force` (* (`KismetMathLibrary.Normal` (`self.Force`)) (`self.MaxForce`)))
      ;[1 1 1] Aplly the force at the point who he interact with the door
      (`PrimitiveComponent.AddForceAtLocation` _sm_door (* (* (`self.Force`) 8.0) (`PrimitiveComponent.GetMass` _sm_door)) (`SceneComponent.K2_GetComponentLocation` (`self.Grab Point Location`)) "None")
      (`KismetSystemLibrary.PrintString` (`KismetStringLibrary.Conv_VectorToString` (`self.Force`)) true true (struct :`G` 0.66 :`B` 1.0 :`A` 1.0) 0.0))))

(event `/Game/Blueprints/BPI/BPI_BP_Door.Grab_Door`
  (params (GrabPoint_Location :type "SceneComponent Object Reference") (`Cam /Camera Arm` :type "CameraComponent Object Reference") (BP_Player_Ref :type "/Game/Blueprints/BP_Player Object Reference"))
  (bind _output_get (set `self.Grab Point Location` GrabPoint_Location))
  (`SceneComponent.K2_AttachToComponent` _output_get (`self.SM_Door`) "None" "KeepWorld" "KeepWorld" "KeepRelative" true)
  (set `self.Cam / Camera Arm` `Cam /Camera Arm`)
  (set `self.PlayerBP_Ref` BP_Player_Ref)
  (set `self.Grabbed` true)
  (set `self.Player Pawn Ref` (`Controller.K2_GetPawn` (`GameplayStatics.GetPlayerController` 0)))
  ;[1 1 1] Block/Slow Movement when Opening the Door
  ;;[1 1 1] Set 0 to block
  (set `CharacterMovementComponent.MaxWalkSpeed` 50.0 (`Character.CharacterMovement` (`GameplayStatics.GetPlayerCharacter` 0))))

(event `Lock look`
  (bind _cam___camera_arm (`self.Cam / Camera Arm`))
  (`SceneComponent.K2_SetWorldRotation` _cam___camera_arm (`KismetMathLibrary.FindLookAtRotation` (`SceneComponent.K2_GetComponentLocation` _cam___camera_arm) (`SceneComponent.K2_GetComponentLocation` (`self.Grab Point Location`))) false false)
  (set `/Game/Blueprints/BP_Player.Grabbing ?` true (`self.PlayerBP_Ref`)))

(fn `UserConstructionScript`)