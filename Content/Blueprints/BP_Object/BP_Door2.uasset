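; Physics door that the player grabs and swings with the mouse, optionally requiring a key from the player's key list.
; Grabbing attaches the grab point to the door mesh and slows walking until release.
; Each tick while held, it locks the view onto that point and turns camera-relative mouse movement into clamped, mass-scaled force applied there.
; A velocity check triggers a one-time creak sound and noise event.
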(event `self.ReceiveTick`
  (params (DeltaSeconds :type "Float (single-precision)"))
  (`self.Force impulse Move`))

(event `Angle Rotation`)

(event `Force impulse Move`
  (bind _returnvalue (`GameplayStatics.GetPlayerController` 0))
  (bind _returnvalue_2 (`self.K2_GetActorLocation`))
  (bind _sm_door (`self.SM_Door`))
  (bind (_deltax _deltay) (`PlayerController.GetInputMouseDelta` _returnvalue))
  (bind _playercameramanager (`PlayerController.PlayerCameraManager` _returnvalue))
  (bind (_relativelocation_x _relativelocation_y _relativelocation_z) (`KismetMathLibrary.BreakVector` (`SceneComponent.RelativeLocation` (`self.DoorHandel`))))
  ;[1 1 1] Recup Mouse Input To Make the Movement
  (if (`self.Grabbed`)
    (`self.Lock look`)
    (set `self.MouseDeltaX` _deltax)
    (set `self.MouseDeltaY` _deltay)
    (bind _output_get (set `self.Force` (+ (* (* (* (`self.GetActorRightVector` _playercameramanager) (`self.MouseDeltaX`)) 100.0) (`PlayerController.GetDeprecatedInputYawScale` _returnvalue)) (* (* (* (`self.GetActorForwardVector` _playercameramanager) (`self.MouseDeltaY`)) 100.0) (* (`PlayerController.GetDeprecatedInputPitchScale` _returnvalue) -1.0)))))
    (set `self.Force` (`KismetMathLibrary.MakeVector` (.x _output_get) (.y _output_get) _relativelocation_z))
    ;[1 1 1] Lock The Max Force
    (if (> (`KismetMathLibrary.Vector_Distance` (`KismetMathLibrary.Vector_Zero`) (`self.Force`)) (`self.MaxForce`))
      (set `self.Force` (* (`KismetMathLibrary.Normal` (`self.Force`)) (`self.MaxForce`)))
      ;[1 1 1] Aplly the force at the point who he interact with the door
      (`PrimitiveComponent.AddForceAtLocation` _sm_door (* (* (`self.Force`) 8.0) (`PrimitiveComponent.GetMass` _sm_door)) (`SceneComponent.K2_GetComponentLocation` (`self.Grab Point Location`)) "None")
      (`KismetSystemLibrary.PrintString` (`KismetStringLibrary.Conv_VectorToString` (`self.Force`)) true true (struct :`G` 0.66 :`B` 1.0 :`A` 1.0) 0.0)
      (bind _returnvalue_3 (`PrimitiveComponent.GetPhysicsLinearVelocity` (`self.SM_Door`) "None"))
      (if (and (> (.x _returnvalue_3) 1.5) (> (.y _returnvalue_3) 1.5))
        (`/Engine/EditorBlueprintResources/StandardMacros.DoOnce` false
          (:`Completed`
            (`GameplayStatics.PlaySoundAtLocation` "/Game/Blueprints/Audio/SFX_Arthur/extras/wav/extra_-_grincement_porte_bois.extra_-_grincement_porte_bois" _returnvalue_2 (struct) 1.0 1.0 0.0 null null null null)
            (`AISense_Hearing.ReportNoiseEvent` _returnvalue_2 1.0 (`GameplayStatics.GetPlayerCharacter` 0) 2000.0)))))))

(event `/Game/Blueprints/BPI/BPI_BP_Door.Grab_Door`
  (params (GrabPoint_Location :type "SceneComponent Object Reference") (`Cam /Camera Arm` :type "CameraComponent Object Reference") (BP_Player_Ref :type "/Game/Blueprints/BP_Player Object Reference"))
  (if (`self.Need Key ?`)
    (`self.Verify Key`)
    (if (`self.HasKey?`)
      (bind _output_get (set `self.Grab Point Location` GrabPoint_Location :!label _label))
      (`SceneComponent.K2_AttachToComponent` _output_get (`self.SM_Door`) "None" "KeepWorld" "KeepWorld" "KeepRelative" true)
      (set `self.Cam / Camera Arm` `Cam /Camera Arm`)
      (set `self.PlayerBP_Ref` BP_Player_Ref)
      (set `self.Grabbed` true)
      (set `self.Player Pawn Ref` (`Controller.K2_GetPawn` (`GameplayStatics.GetPlayerController` 0)))
      ;[1 1 1] Block/Slow Movement when Opening the Door
      ;;[1 1 1] Set 0 to block
      (set `CharacterMovementComponent.MaxWalkSpeed` 50.0 (`Character.CharacterMovement` (`GameplayStatics.GetPlayerCharacter` 0))))
    (else
      (set `self.HasKey?` true)
      (goto _label))))

(event `Verify Key`
  (bind _asbp_player (cast `/Game/Blueprints/BP_Player` (`GameplayStatics.GetPlayerCharacter` 0)))
  (for _array_element (`/Game/Blueprints/BP_Player.List of key` _asbp_player)
    (if (== _array_element (`self.Key Needed`))
      (set `self.HasKey?` true))))

(event `Lock look`
  (`Controller.SetControlRotation` (`GameplayStatics.GetPlayerController` 0) (`KismetMathLibrary.FindLookAtRotation` (`SceneComponent.K2_GetComponentLocation` (`self.Cam / Camera Arm`)) (`SceneComponent.K2_GetComponentLocation` (`self.Grab Point Location`))))
  (set `/Game/Blueprints/BP_Player.Grabbing ?` true (`self.PlayerBP_Ref`))
  (`KismetSystemLibrary.PrintString` "Hello"))

(event `/Game/Blueprints/BPI/BPI_BP_Door.Release_Door`
  (set `self.Grabbed` false)
  (set `/Game/Blueprints/BP_Player.Grabbing ?` false (`self.PlayerBP_Ref`))
  (set `CharacterMovementComponent.MaxWalkSpeed` 275.0 (`Character.CharacterMovement` (`GameplayStatics.GetPlayerCharacter` 0))))

(fn `UserConstructionScript`)