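; BP_Door2 is a physics door that the player grabs and swings with mouse movement.
; GrabDoor flags the grab, caches the pawn and slows the character's walk speed.
; While grabbed, Tick builds a force from camera-relative mouse deltas plus pawn velocity, using the handle's relative Z.
; Only when that force exceeds MaxForce is it clamped, applied to the door mesh scaled by mass, and debug-printed.
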(event `self.ReceiveTick`
  (params (DeltaSeconds :type "Float (single-precision)"))
  (bind _returnvalue (`GameplayStatics.GetPlayerController` 0))
  (bind _sm_door (`self.SM_Door`))
  (bind (_deltax _deltay) (`PlayerController.GetInputMouseDelta` _returnvalue))
  (bind _playercameramanager (`PlayerController.PlayerCameraManager` _returnvalue))
  (bind (_relativelocation_x _relativelocation_y _relativelocation_z) (`KismetMathLibrary.BreakVector` (`SceneComponent.RelativeLocation` (`self.DoorHandel`))))
  ;[1 1 1] Recup Mouse Input To Make the Movement
  (if (`self.Grabbed`)
    (set `self.MouseDeltaX` _deltax)
    (set `self.MouseDeltaY` _deltay)
    (bind _output_get (set `self.Force` (+ (* (* (* (`self.GetActorRightVector` _playercameramanager) (`self.MouseDeltaX`)) 200.0) (`PlayerController.GetDeprecatedInputYawScale` _returnvalue)) (* (* (* (`self.GetActorForwardVector` _playercameramanager) (`self.MouseDeltaY`)) 300.0) (* (`PlayerController.GetDeprecatedInputPitchScale` _returnvalue) -1.0)))))
    ;[1 1 1] Use The player Movement (Velocity)
    (bind _output_get_2 (set `self.Force` (+ _output_get (* (`self.GetVelocity` (`self.Player Pawn Ref`)) 0.8))))
    (set `self.Force` (`KismetMathLibrary.MakeVector` (.x _output_get_2) (.y _output_get_2) _relativelocation_z))
    ;[1 1 1] Lock The Max Force
    (if (> (`KismetMathLibrary.Vector_Distance` (`KismetMathLibrary.Vector_Zero`) (`self.Force`)) (`self.MaxForce`))
      (set `self.Force` (* (`KismetMathLibrary.Normal` (`self.Force`)) (`self.MaxForce`)))
      (`PrimitiveComponent.AddForce` _sm_door (* (* (`self.Force`) 8.0) (`PrimitiveComponent.GetMass` _sm_door)) "None" false)
      (`KismetSystemLibrary.PrintString` (`KismetStringLibrary.Conv_VectorToString` (`self.Force`)) true true (struct :`G` 0.66 :`B` 1.0 :`A` 1.0) 0.0))))

(event `/Game/Blueprints/BPI/BPI_BP_Door.Grab_Door`
  (set `self.Grabbed` true)
  (set `self.Player Pawn Ref` (`Controller.K2_GetPawn` (`GameplayStatics.GetPlayerController` 0)))
  ;[1 1 1] Block/Slow Movement when Opening the Door
  ;;[1 1 1] Set 0 to block
  (set `CharacterMovementComponent.MaxWalkSpeed` 50.0 (`Character.CharacterMovement` (`GameplayStatics.GetPlayerCharacter` 0))))

(fn `UserConstructionScript`)