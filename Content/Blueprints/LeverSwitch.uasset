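; LeverSwitch is a physics lever actor that switches a linked object on or off.
; Each tick it reads the handle's pitch in actor-local space and compares it to a threshold.
; The result sets the physics constraint's angular orientation target, snapping the handle toward one of two rest angles.
; It also sends the activate or deactivate message to LinkedObject on every check, not only on state changes.
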(event `self.ReceiveTick`
  (params (DeltaSeconds :type "Float (single-precision)"))
  (`self.Lever_Check`))

(event `Lever_Check`
  (bind _linkedobject (`self.LinkedObject`))
  (bind _returnvalue (< (.pitch (`KismetMathLibrary.InverseTransformRotation` (`self.GetTransform`) (`SceneComponent.K2_GetComponentRotation` (`self.Handle`)))) 20.0))
  (`PhysicsConstraintComponent.SetAngularOrientationTarget` (`self.PhysicsConstraint`) (`KismetMathLibrary.MakeRotator` 0.0 (`KismetMathLibrary.SelectFloat` -45.0 45.0 _returnvalue)))
  (if _returnvalue
    (message `/Game/Blueprints/BPI/BPI_LeverActivate.Lever_Activate` _linkedobject)
    (else
      (message `/Game/Blueprints/BPI/BPI_Lever_Desactivate.Lever_Desactivate` _linkedobject))))

(fn `UserConstructionScript`)