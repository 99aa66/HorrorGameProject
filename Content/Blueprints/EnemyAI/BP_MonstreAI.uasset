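; Monster enemy character that runs a Search, Patrol or Guard behavior tree chosen by AIType.
; Seeing the player fills a detection timeline, or triggers instantly, to start a faster chase with cry and music; a retriggerable delay after the last sighting reverses it.
; Heard noises set a blackboard investigation flag unless already chasing.
; Getters expose guard post, noise location and index-matched patrol points.
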(event `self.ReceiveBeginPlay`
  (bind _ai_controller_ref (`self.AI Controller REF`))
  (`|ExecutionSequence`
    (:`then_0`
      ;[1 1 1] Set AI type
      (set `self.AI Controller REF` (`AIBlueprintHelperLibrary.GetAIController` self))
      (switch `/Game/Blueprints/Enum/E_AI_Type` (`self.AI Type`)
        (:`NewEnumerator0`
          (`AIController.RunBehaviorTree` _ai_controller_ref "/Game/Blueprints/EnemyAI/BT/BT_SAI_Search.BT_SAI_Search"))
        (:`NewEnumerator1`
          (`AIController.RunBehaviorTree` _ai_controller_ref "/Game/Blueprints/EnemyAI/BT/BT_SAI_Patrol.BT_SAI_Patrol"))
        (:`NewEnumerator2`
          (`AIController.RunBehaviorTree` (`self.AI Controller REF`) "/Game/Blueprints/EnemyAI/BT/BT_SAI_Guard.BT_SAI_Guard"))))
    (:`then_1`
      ;[1 1 1] Set guard post position
      (set `self.GuardPostPosition` (`KismetMathLibrary.SelectVector` (`self.K2_GetActorLocation`) (`self.GuardPostPosition`) (`self.Use Current Position?`))))
    (:`then_2`
      ;[1 1 1] Set the detection time
      (`TimelineComponent.SetPlayRate` (`self.Fill Detection Meter`) (/ 1.0 (`self.Detection Time`))))))

(event `self.PawnSensing.OnSeePawn`
  (params (Pawn :type "Pawn Object Reference"))
  (bind _charactermovement (`self.CharacterMovement`))
  (bind _returnvalue (`AIBlueprintHelperLibrary.GetBlackboard` (`self.AI Controller REF`)))
  ;[1 1 1] Detect player
  (if (== Pawn (`GameplayStatics.GetPlayerCharacter` 0))
    (`|ExecutionSequence`
      (:`then_0`
        ;;[1 1 1] Fill up/drain detection meter
        (if (`self.Detect Immediately`)
          ;;[1 1 1] Start chasing
          (`BlackboardComponent.SetValueAsBool` _returnvalue "CanSeePlayer?" true :!label _label)
          (set `CharacterMovementComponent.MaxWalkSpeed` 300.0 _charactermovement)
          (set `self.IsChasing?` true)
          (`/Engine/EditorBlueprintResources/StandardMacros.DoOnce` false :!label _label_2
            (:`Completed`
              (`GameplayStatics.PlaySoundAtLocation` "/Game/Blueprints/Audio/SFX_Arthur/monstre/wav/monstre_-_cri_1.monstre_-_cri_1" (`self.K2_GetActorLocation`) (struct) 1.0 1.0 0.0 null null null null)
              (message `/Game/Blueprints/BPI/BPI_StealthAI.Start Chase Music` (`GameplayStatics.GetGameInstance`))))
          (else
            (`|ExecutionSequence`
              (:`then_0`
                (bind _direction (`Timeline|Fill Detection Meter` :!label _label_3)
                  (:`Finished`
                    (switch `ETimelineDirection` _direction
                      (:`Forward`
                        (goto _label))
                      (:`Backward`
                        ;;[1 1 1] Stop chasing
                        (`BlackboardComponent.SetValueAsBool` _returnvalue "CanSeePlayer?" false :!label _label_4)
                        (set `CharacterMovementComponent.MaxWalkSpeed` 150.0 _charactermovement)
                        (set `self.IsChasing?` false)
                        (message `/Game/Blueprints/BPI/BPI_StealthAI.Stop Chase Music` (`GameplayStatics.GetGameInstance`))
                        (goto _label_2 :!via `Reset`))))))
              (:`then_1`
                (`/Engine/EditorBlueprintResources/StandardMacros.DoOnce` false :!label _label_5
                  (:`Completed`
                    (`GameplayStatics.PlaySoundAtLocation` "/Game/Blueprints/Audio/SFX_Arthur/monstre/wav/monstre-respiration-2.monstre-respiration-2" (`self.K2_GetActorLocation`) (struct) 1.0 1.0 0.0 null null null null))))))))
      (:`then_1`
        (`KismetSystemLibrary.RetriggerableDelay` (`self.Search Time`))
        (if (`self.Detect Immediately`)
          (goto _label_4)
          (else
            (`TimelineComponent.Stop` (`self.Fill Detection Meter`))
            (`|ExecutionSequence`
              (:`then_0`
                (goto _label_5 :!via `Reset`))
              (:`then_1`
                (goto _label_3 :!via `Reverse`)))))))))

(event `self.AIPerception.OnTargetPerceptionUpdated`
  (params (Actor :type "Actor Object Reference") (Stimulus :type "AIStimulus Structure"))
  (bind ((`StimulusLocation` _stimuluslocation) (`bSuccessfullySensed` _bsuccessfullysensed)) (break `AIStimulus` Stimulus))
  ;[1 1 1] Investigate any noise heard
  (if _bsuccessfullysensed
    (set `self.Noise Location` _stimuluslocation)
    (if (not (`self.IsChasing?`))
      (`BlackboardComponent.SetValueAsBool` (`AIBlueprintHelperLibrary.GetBlackboard` (`self.AI Controller REF`)) "HeardNoise?" true)
      ;;[1 1 1] Sound when he heard a Noise
      (`GameplayStatics.PlaySoundAtLocation` "/Game/Blueprints/Audio/SFX_Arthur/monstre/wav/monstre-respiration-1.monstre-respiration-1" (`self.K2_GetActorLocation`) (struct) 1.0 1.0 0.0 null null null null))))

(event `/Game/Blueprints/BPI/BPI_StealthAI.EndInvestigation`
  ;[1 1 1] Investigate any noise heard
  (`BlackboardComponent.SetValueAsBool` (`AIBlueprintHelperLibrary.GetBlackboard` (`self.AI Controller REF`)) "HeardNoise?" false))

(fn `GetGuardPost`
  (returns (Location :type "Vector Structure"))
  (return (`self.GuardPostPosition`)))

(fn `GetNoiseLocation`
  (returns (Location :type "Vector Structure"))
  (return (`self.Noise Location`)))

(fn `GetpatrolPoints`
  (returns (`Patrol Path` :type "Array of /Game/Blueprints/EnemyAI/BP_PatrolPoint Object Reference"))
  ;[1 1 1] Get the patrol points on the desired patrol path
  (bind _outactors (`GameplayStatics.GetAllActorsOfClass` "/Game/Blueprints/EnemyAI/BP_PatrolPoint.BP_PatrolPoint_C"))
  (for _array_element _outactors
    (if (== (`/Game/Blueprints/EnemyAI/BP_PatrolPoint.Patrol Path Index` _array_element) (`self.Patrol Path Index`))
      (`KismetArrayLibrary.Array_Add` (`self.Patrol Path`) _array_element)))
  (return (`self.Patrol Path`)))

(fn `UserConstructionScript`)